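; Base projectile Blueprint that handles the sound and visual effects for a projectile's spawn, flight and impact.
; BeginPlay plays the spawn sound, attaches the flying sound to the root and spawns a muzzle effect facing the actor's forward vector.
; OnSpawnProjectileHitFX plays the impact sound and effect at a supplied hit location.
; Each asset is validity-checked first, and the graph contains no movement, collision or damage logic.
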(event EventBeginPlay
  (Utilities|FlowControl|Sequence
    (:then_0
      (bind _projectilespawnsound (Variables|Default|GetProjectileSpawnSound)
        (:then
          (Audio|PlaySoundatLocation _projectilespawnsound (Transformation|GetActorLocation) "0, 0, 0" 1.0 1.0 0.0 0 0 0 0))
        (:else)))
    (:then_1
      (bind _projectileflyingsound (Variables|Default|GetProjectileFlyingSound)
        (:then
          (Audio|SpawnSoundAttached _projectileflyingsound (Variables|Transformation|GetRootComponent) "None" "0, 0, 0" "0, 0, 0" "KeepRelativeOffset" true 1.0 1.0 0.0 0 0))
        (:else)))
    (:then_2
      (bind _projectilemuszzkefx (Variables|Default|GetProjectileMuszzkeFX)
        (:then
          (Niagara|SpawnSystematLocation _projectilemuszzkefx (Transformation|GetActorLocation) (Math|Conversions|RotationFromXVector (Transformation|GetActorForwardVector))))
        (:else)))))

(event EventOnSpawnProjectileHitFX
  (params (HitLocation :type Vector%20%28by%20ref%29 :default "0, 0, 0"))
  (Utilities|FlowControl|Sequence
    (:then_0
      (bind _projectileimpactsound (Variables|Default|GetProjectileImpactSound)
        (:then
          (Audio|PlaySoundatLocation _projectileimpactsound HitLocation "0, 0, 0" 1.0 1.0 0.0 0 0 0 0))
        (:else)))
    (:then_1
      (bind _projectile_impact_efffects (Variables|Default|GetProjectile%20Impact%20Efffects)
        (:then
          (Niagara|SpawnSystematLocation _projectile_impact_efffects HitLocation))
        (:else)))))

(fn ConstructionScript)